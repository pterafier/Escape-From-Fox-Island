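; AI controller for a fox that wanders at random and flees when attacked.
; Two looping timers started on BeginPlay drive it: Patrol moves a stationary pawn to a random reachable point nearby.
; Panic checks the Attacked and IsDead flags, which are not set here, and moves to a random point in a wider radius.
; Starting a panic move cancels patrol permanently, and the panic timer clears only if IsDead is set.
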(event Custom|Panic
  (if (and (not (Variables|Default|GetisDead)) (Variables|Default|GetAttacked))
    (AI|AIMoveTo 0 (.RandomLocation (AI|Navigation|GetRandomReachablePointinRadius (Transformation|GetActorLocation) 2.5e+03 0 0)) 0 5.0 false
      (:then
        (Utilities|Time|ClearandInvalidateTimerbyHandle (stale EventBeginPlay _returnvalue))
        (if (Variables|Default|GetisDead)
          (Utilities|Time|ClearandInvalidateTimerbyHandle (stale EventBeginPlay _returnvalue_2)))))))

(event Custom|Patrol
  (if (not (> (Math|Vector|VectorLength (Transformation|GetVelocity (Pawn|GetControlledPawn))) 0.0))
    (AI|AIMoveTo 0 (.RandomLocation (AI|Navigation|GetRandomReachablePointinRadius (Transformation|GetActorLocation) 1.5e+03 0 0)) 0 2e+01 false)))

(event EventBeginPlay
  (bind _returnvalue (Utilities|Time|SetTimerbyEvent (delegate Custom|Patrol) 5.0 true))
  (bind _returnvalue_2 (Utilities|Time|SetTimerbyEvent (delegate Custom|Panic) 2.0 true)))

(fn ConstructionScript)