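; Huntable fox character that can be killed and then skinned for a hide.
; Damage flags its anim Blueprint and AI controller, raises walk speed, and activates a particle effect if the player's equipped weapon is a lit torch.
; At zero health it plays a death animation and stops moving.
; The next hit plays blood effects, credits a hide, flags inventory widgets and shrinks the capsule via timeline, but DestroyActor is never reached.
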(event Custom|OnTakeAnyDamage_Event
  (params (DamagedActor :type Actor%20Object%20Reference) (Damage :type Float%20%28single-precision%29) (DamageType :type Damage%20Type%20Object%20Reference) (InstigatedBy :type Controller%20Object%20Reference) (DamageCauser :type Actor%20Object%20Reference))
  (bind _particlesystem (Variables|Default|GetParticleSystem))
  (bind _as_bp_sword_character (Variables|Default|GetAs%20BP%20Sword%20Character))
  (bind _capsulecomponent (Variables|Collision|GetCapsuleComponent))
  (if (not (Variables|Default|GetisDead))
    (bind _asabp_fox (Utilities|Casting|CastToABP_Fox (Components|SkeletalMesh|GetAnimInstance (Variables|Character|GetMesh))))
    (bind _asbp_fox_controller (Utilities|Casting|CastToBP_FoxController (AI|GetAIController self)))
    (Variables|/Game/AI/ABP_Fox.ABP_Fox_C|SetIsAttacked _asabp_fox true)
    (Variables|/Game/AI/BP_FoxController.BP_FoxController_C|SetAttacked _asbp_fox_controller true)
    (if (and (Utilities|Enum|Equal(Enum) (Variables|/Game/FPSwordAndShield/Blueprints/BP_SwordCharacter.BP_SwordCharacter_C|GetEquippedWeapon _as_bp_sword_character) "NewEnumerator0") (Variables|/Game/FPSwordAndShield/Blueprints/BP_SwordCharacter.BP_SwordCharacter_C|GetTorchLit _as_bp_sword_character))
      (Components|Activation|Activate _particlesystem false))
    (Variables|Default|SetHealth (- (Variables|Default|GetHealth) Damage))
    (Variables|/Script/Engine.CharacterMovementComponent|SetMaxWalkSpeed (Variables|Character|GetCharacterMovement) 1.1e+03)
    (if (<= (Variables|Default|GetHealth) 0.0)
      (Variables|/Game/AI/BP_FoxController.BP_FoxController_C|SetisDead _asbp_fox_controller true)
      (Variables|Default|SetisDead true)
      (Components|Activation|Deactivate _particlesystem)
      (Components|Animation|PlayAnimation (Variables|Character|GetMesh) "/Game/AnimalVarietyPack/Fox/Animations/ANIM_Fox_Death.ANIM_Fox_Death" false)
      (Pawn|Components|CharacterMovement|DisableMovement (Variables|Character|GetCharacterMovement)))
    (else
      (Utilities|FlowControl|DoOnce false
        (:Completed
          (Effects|SpawnEmitteratLocation "/Game/Realistic_Starter_VFX_Pack_Vol2/Particles/Blood/P_Blood_Splat_Cone.P_Blood_Splat_Cone" (- (Transformation|GetActorLocation) "0.000000,0.000000,20.000000"))
          (Audio|PlaySound2D "/Game/Audio/SC_BloodSpurt.SC_BloodSpurt" (Math|Random|RandomFloatinRange 0.7 1.1) (Math|Random|RandomFloatinRange 0.9 1.1) 0.0 0 0 false)
          (Math|Integer|IncrementInt (Variables|/Game/FPSwordAndShield/Blueprints/BP_SwordCharacter.BP_SwordCharacter_C|GetHide (Variables|Default|GetAs%20BP%20Sword%20Character))
            (:%20%20
              (bind _foundwidgets (Widget|GetAllWidgetsOfClass "/Game/UI/WB_Inventory_.WB_Inventory__C" true))
              (for _array_element _foundwidgets
                (Variables|/Game/UI/WB_Inventory_.WB_Inventory__C|SetHideCollected _array_element true)
                (Collision|SetCollisionEnabled (Variables|Collision|GetCapsuleComponent) "NoCollision")
                (Utilities|FlowControl|Delay 0.25)
                (bind _newtrack_0 (Timeline|Timeline Play)
                  (:Update
                    (Transformation|SetWorldScale3D _capsulecomponent (Math|Vector|Lerp(Vector) (Transformation|GetWorldScale _capsulecomponent) "0, 0, 0" _newtrack_0))
                    (Utilities|FlowControl|Delay 1.0)))))))))))

(event EventBeginPlay
  (EventDispatchers|AssignOnTakeAnyDamage (delegate Custom|OnTakeAnyDamage_Event))
  (bind _asbp_sword_character (Utilities|Casting|CastToBP_SwordCharacter (Game|GetPlayerCharacter 0)))
  (Variables|Default|SetAs%20BP%20Sword%20Character _asbp_sword_character))

(fn ConstructionScript)