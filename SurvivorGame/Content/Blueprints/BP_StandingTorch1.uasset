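; BP_StandingTorch1 is a standing torch that lights when it takes any damage.
; Damage activates its particle system, shows its point light and sets TorchLit.
; The particle system's activation event passes through a DoOnce to increment TorchesLit on the BP_TorchManager found in the level, so the torch is counted only once.
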(event OnComponentActivated(ParticleSystem)
  (params (Component :type Actor%20Component%20Object%20Reference) (bReset :type Boolean))
  (Utilities|FlowControl|DoOnce false
    (:Completed
      (bind _returnvalue (Actor|GetActorOfClass "/Game/Blueprints/BP_TorchManager.BP_TorchManager_C"))
      (Math|Integer|IncrementInt (Variables|/Game/Blueprints/BP_TorchManager.BP_TorchManager_C|GetTorchesLit _returnvalue)))))

(event Custom|OnTakeAnyDamage_Event
  (params (DamagedActor :type Actor%20Object%20Reference) (Damage :type Float%20%28single-precision%29) (DamageType :type Damage%20Type%20Object%20Reference) (InstigatedBy :type Controller%20Object%20Reference) (DamageCauser :type Actor%20Object%20Reference))
  (Components|Activation|Activate (Variables|Default|GetParticleSystem) false)
  (Rendering|SetVisibility (Variables|Default|GetPointLight) true false)
  (Variables|Default|SetTorchLit true))

(event EventBeginPlay
  (EventDispatchers|AssignOnTakeAnyDamage (delegate Custom|OnTakeAnyDamage_Event)))

(event Collision|EventActorBeginOverlap
  (params (OtherActor :type Actor%20Object%20Reference)))

(event EventTick
  (params (DeltaSeconds :type Float%20%28single-precision%29)))

(fn ConstructionScript)