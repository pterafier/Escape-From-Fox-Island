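; BP_Stick is a collectible stick that shows a tip text when the player's BP_SwordCharacter enters its Box trigger.
; A looping timer keeps the tip rotated toward the player, and the Box overlap events show and hide it.
; PickupStick flags the stick as collected in WB_Inventory_ widgets, increments the character's stick count, plays a randomly varied pickup sound and destroys the actor.
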(event OnComponentBeginOverlap(Box)
  (params (OverlappedComponent :type Primitive%20Component%20Object%20Reference) (OtherActor :type Actor%20Object%20Reference) (OtherComp :type Primitive%20Component%20Object%20Reference) (OtherBodyIndex :type Integer) (bFromSweep :type Boolean) (SweepResult :type Hit%20Result%20Structure%20%28by%20ref%29))
  ;[1 1 1] When player is close, show text. hide text when they leave range
  (if (== OtherActor (Variables|Default|GetAs%20BP%20Sword%20Character))
    (Development|SetHiddeninGame (Variables|Default|GetTipText) false false)))

(event OnComponentEndOverlap(Box)
  (params (OverlappedComponent :type Primitive%20Component%20Object%20Reference) (OtherActor :type Actor%20Object%20Reference) (OtherComp :type Primitive%20Component%20Object%20Reference) (OtherBodyIndex :type Integer))
  ;[1 1 1] When player is close, show text. hide text when they leave range
  (if (== OtherActor (Variables|Default|GetAs%20BP%20Sword%20Character))
    (Development|SetHiddeninGame (Variables|Default|GetTipText) true false)))

(event Custom|TextLookAtPlayer
  ;[1 1 1] Initializes player referennce, hides tip text, sets tip text to look at player
  (Transformation|SetWorldRotation (Variables|Default|GetTipText) (Math|Rotator|FindLookatRotation (Transformation|GetWorldLocation (Variables|Default|GetTipText)) (Transformation|GetActorLocation (stale EventBeginPlay _output_get))) false false))

(event EventPickupStick
  (bind _foundwidgets (Widget|GetAllWidgetsOfClass "/Game/UI/WB_Inventory_.WB_Inventory__C" true))
  (for _array_element _foundwidgets
    (Variables|/Game/UI/WB_Inventory_.WB_Inventory__C|SetStickCollected _array_element true))
  (Math|Integer|IncrementInt (Variables|/Game/FPSwordAndShield/Blueprints/BP_SwordCharacter.BP_SwordCharacter_C|GetSticksQuantity (Variables|Default|GetAs%20BP%20Sword%20Character))
    (:%20%20
      (Audio|PlaySound2D "/Game/Audio/SC_Pickup.SC_Pickup" (Math|Random|RandomFloatinRange 0.8 1.1) (Math|Random|RandomFloatinRange 0.8 1.1) 0.0 0 0)
      (Development|PrintString "Picked up stick")
      (Actor|DestroyActor))))

(event EventBeginPlay
  ;[1 1 1] Initializes player referennce, hides tip text, sets tip text to look at player
  (bind _asbp_sword_character (Utilities|Casting|CastToBP_SwordCharacter (Game|GetPlayerCharacter 0)))
  (bind _output_get (Variables|Default|SetAs%20BP%20Sword%20Character _asbp_sword_character))
  (Development|SetHiddeninGame (Variables|Default|GetTipText) true false)
  (Utilities|Time|SetTimerbyEvent (delegate Custom|TextLookAtPlayer) 0.08 true))

(fn ConstructionScript)