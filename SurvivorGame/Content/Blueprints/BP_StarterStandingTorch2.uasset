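; Standing starter torch that, judging by its logic, handles lighting the player's hand torch and feeds the torch-lit count.
; On taking damage, it casts the damaged actor to BP_HandTorch, turns on that torch's particles and light, plays a combust sound and sets TorchLit on the cached BP_SwordCharacter.
; Separately, the first activation of its own particle system increments TorchesLit on BP_TorchManager through a DoOnce.
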(event OnComponentActivated(ParticleSystem)
  (params (Component :type Actor%20Component%20Object%20Reference) (bReset :type Boolean))
  (Utilities|FlowControl|DoOnce false
    (:Completed
      (bind _returnvalue (Actor|GetActorOfClass "/Game/Blueprints/BP_TorchManager.BP_TorchManager_C"))
      (Math|Integer|IncrementInt (Variables|/Game/Blueprints/BP_TorchManager.BP_TorchManager_C|GetTorchesLit _returnvalue)))))

(event Custom|OnTakeAnyDamage_Event
  (params (DamagedActor :type Actor%20Object%20Reference) (Damage :type Float%20%28single-precision%29) (DamageType :type Damage%20Type%20Object%20Reference) (InstigatedBy :type Controller%20Object%20Reference) (DamageCauser :type Actor%20Object%20Reference))
  (bind _asbp_hand_torch (Utilities|Casting|CastToBP_HandTorch DamagedActor))
  (Components|Activation|Activate (Variables|/Game/Blueprints/BP_HandTorch.BP_HandTorch_C|GetParticleSystem _asbp_hand_torch) false)
  (Rendering|SetVisibility (Variables|/Game/Blueprints/BP_HandTorch.BP_HandTorch_C|GetPointLight _asbp_hand_torch) true false)
  (Audio|PlaySound2D "/Game/Audio/Fire_Combust.Fire_Combust" 0.8 0.8 0.0 0 0)
  (Variables|/Game/FPSwordAndShield/Blueprints/BP_SwordCharacter.BP_SwordCharacter_C|SetTorchLit (stale EventBeginPlay _asbp_sword_character) true))

(event EventBeginPlay
  (EventDispatchers|AssignOnTakeAnyDamage (delegate Custom|OnTakeAnyDamage_Event))
  (bind _asbp_sword_character (Utilities|Casting|CastToBP_SwordCharacter (Game|GetPlayerCharacter 0))))

(event Collision|EventActorBeginOverlap
  (params (OtherActor :type Actor%20Object%20Reference)))

(event EventTick
  (params (DeltaSeconds :type Float%20%28single-precision%29)))

(fn ConstructionScript)