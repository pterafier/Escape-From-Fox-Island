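; Campfire actor that lights once when it first takes any damage and lets the player regenerate hunger nearby.
; Ignition activates the particles and light, plays fire sounds, removes cold warning widgets and immediately enables the player's hunger regeneration.
; Once lit, the sphere's begin and end overlap events toggle CanRegenHunger on the cached BP_SwordCharacter.
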(event OnComponentBeginOverlap(Sphere)
  (params (OverlappedComponent :type Primitive%20Component%20Object%20Reference) (OtherActor :type Actor%20Object%20Reference) (OtherComp :type Primitive%20Component%20Object%20Reference) (OtherBodyIndex :type Integer) (bFromSweep :type Boolean) (SweepResult :type Hit%20Result%20Structure%20%28by%20ref%29))
  (if (and (== OtherActor (Variables|Default|GetAs%20BP%20Sword%20Character)) (Variables|Default|GetFireActivated))
    (Variables|/Game/FPSwordAndShield/Blueprints/BP_SwordCharacter.BP_SwordCharacter_C|SetCanRegenHunger (Variables|Default|GetAs%20BP%20Sword%20Character) true)))

(event OnComponentEndOverlap(Sphere)
  (params (OverlappedComponent :type Primitive%20Component%20Object%20Reference) (OtherActor :type Actor%20Object%20Reference) (OtherComp :type Primitive%20Component%20Object%20Reference) (OtherBodyIndex :type Integer))
  (if (and (== OtherActor (Variables|Default|GetAs%20BP%20Sword%20Character)) (Variables|Default|GetFireActivated))
    (Variables|/Game/FPSwordAndShield/Blueprints/BP_SwordCharacter.BP_SwordCharacter_C|SetCanRegenHunger (Variables|Default|GetAs%20BP%20Sword%20Character) false)))

(event Custom|OnTakeAnyDamage_Event
  (params (DamagedActor :type Actor%20Object%20Reference) (Damage :type Float%20%28single-precision%29) (DamageType :type Damage%20Type%20Object%20Reference) (InstigatedBy :type Controller%20Object%20Reference) (DamageCauser :type Actor%20Object%20Reference))
  (Utilities|FlowControl|DoOnce false
    (:Completed
      (Components|Activation|Activate (Variables|Default|GetParticleSystem) false)
      (Rendering|SetVisibility (Variables|Default|GetPointLight) true false)
      (Variables|/Game/FPSwordAndShield/Blueprints/BP_SwordCharacter.BP_SwordCharacter_C|SetCanRegenHunger (Variables|Default|GetAs%20BP%20Sword%20Character) true)
      (Variables|Default|SetFireActivated true)
      (Variables|Default|SetPlayerInRange true)
      (Audio|PlaySoundatLocation "/Game/Audio/363093__thewoodlandnomad__fire-crackle-and-flames-001.363093__thewoodlandnomad__fire-crackle-and-flames-001" (Transformation|GetActorLocation) "0, 0, 0" 1.0 1.0 0.0 "/Game/Audio/NewSoundAttenuation.NewSoundAttenuation" 0 0 0)
      (Audio|PlaySound2D "/Game/Audio/Fire_Combust.Fire_Combust" 0.8 0.8 0.0 0 0)
      (bind _foundwidgets (Widget|GetAllWidgetsOfClass "/Game/UI/WB_ColdWarning.WB_ColdWarning_C" true))
      (for _array_element _foundwidgets
        (Widget|RemovefromParent _array_element)
        (Utilities|Platform|CollectGarbage)))))

(event EventBeginPlay
  (EventDispatchers|AssignOnTakeAnyDamage (delegate Custom|OnTakeAnyDamage_Event))
  (bind _asbp_sword_character (Utilities|Casting|CastToBP_SwordCharacter (Game|GetPlayerCharacter 0)))
  (Variables|Default|SetAs%20BP%20Sword%20Character _asbp_sword_character))

(event Collision|EventActorBeginOverlap
  (params (OtherActor :type Actor%20Object%20Reference)))

(event EventTick
  (params (DeltaSeconds :type Float%20%28single-precision%29)))

(fn ConstructionScript)