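; BP_TorchManager watches for all goal torches being lit and then triggers an easter egg ending.
; A looping timer started on BeginPlay compares TorchesLit to GoalTorches, then clears itself and fires once on a match.
; A timeline eases global time dilation into slow motion, then shows the WB_GameOver widget and plays a boat rescue sound.
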(event Custom|EasterEgg
  (if (== (Variables|Default|GetTorchesLit) (Variables|Default|GetGoalTorches))
    (Utilities|Time|ClearandInvalidateTimerbyHandle (stale EventBeginPlay _returnvalue))
    (Utilities|FlowControl|DoOnce false
      (:Completed
        (Variables|Default|SetEasterEggUnlocked true)
        (bind _newtrack_0 (Timeline|Timeline Play)
          (:Update
            (Utilities|Time|SetGlobalTimeDilation (Math|Float|Lerp 1.0 0.25 _newtrack_0)))
          (:Finished
            (bind _returnvalue (UserInterface|CreateWidget "/Game/UI/Menus/WB_GameOver.WB_GameOver_C"))
            (UserInterface|Viewport|AddtoViewport _returnvalue 0)
            (Audio|PlaySound2D "/Game/Audio/EasterEggBoatRescueSound.EasterEggBoatRescueSound" 1.0 1.0 0.0 0 0)))))))

(event EventBeginPlay
  (bind _returnvalue (Utilities|Time|SetTimerbyEvent (delegate Custom|EasterEgg) 0.1 true)))

(fn ConstructionScript)