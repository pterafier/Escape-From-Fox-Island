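; Choppable tree actor that takes damage and yields a log to the player's BP_SwordCharacter when felled.
; Each hit waits briefly, then lowers Health and plays a randomized chop sound.
; At zero Health, a DoOnce increments Logs, plays a whoosh and effect, and hides the mesh and disables collision.
; It flags WB_Inventory_ widgets as LogCollected, with delayed destruction triggered inside that widget loop.
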(event Custom|OnTakeAnyDamage_Event
  (params (DamagedActor :type Actor%20Object%20Reference) (Damage :type Float%20%28single-precision%29) (DamageType :type Damage%20Type%20Object%20Reference) (InstigatedBy :type Controller%20Object%20Reference) (DamageCauser :type Actor%20Object%20Reference))
  (Utilities|FlowControl|Delay 0.2)
  (Variables|Default|SetHealth (- (Variables|Default|GetHealth) Damage))
  (Audio|PlaySound2D "/Game/Audio/SC_WoodChop.SC_WoodChop" (Math|Random|RandomFloatinRange 0.8 1.2) (Math|Random|RandomFloatinRange 0.9 1.1) 0.0 0 0)
  (if (<= (Variables|Default|GetHealth) 0.0)
    (Utilities|FlowControl|DoOnce false
      (:Completed
        (Audio|PlaySound2D "/Game/Magic___Spell_Sounds_PRO/General/wav/Magic_Whoosh_3.Magic_Whoosh_3" (Math|Random|RandomFloatinRange 1.0 1.2) (Math|Random|RandomFloatinRange 1.0 1.15) 0.1 0 0)
        (Math|Integer|IncrementInt (Variables|/Game/FPSwordAndShield/Blueprints/BP_SwordCharacter.BP_SwordCharacter_C|GetLogs (Variables|Default|GetAs%20BP%20Sword%20Character))
          (:%20%20
            (Components|Activation|Activate (Variables|Default|GetFire_Grd_02) false)
            (Development|SetHiddeninGame (Variables|Default|GetStaticMesh) true true)
            (Collision|SetCollisionEnabled (Variables|Default|GetStaticMesh) "NoCollision")
            (bind _foundwidgets (Widget|GetAllWidgetsOfClass "/Game/UI/WB_Inventory_.WB_Inventory__C" true))
            (for _array_element _foundwidgets
              (Variables|/Game/UI/WB_Inventory_.WB_Inventory__C|SetLogCollected _array_element true)
              (Utilities|FlowControl|Delay 5.0)
              (Actor|DestroyActor))))))))

(event EventBeginPlay
  (bind _asbp_sword_character (Utilities|Casting|CastToBP_SwordCharacter (Game|GetPlayerCharacter 0)))
  (Variables|Default|SetAs%20BP%20Sword%20Character _asbp_sword_character)
  (EventDispatchers|AssignOnTakeAnyDamage (delegate Custom|OnTakeAnyDamage_Event)))

(event Collision|EventActorBeginOverlap
  (params (OtherActor :type Actor%20Object%20Reference)))

(event EventTick
  (params (DeltaSeconds :type Float%20%28single-precision%29)))

(fn ConstructionScript)