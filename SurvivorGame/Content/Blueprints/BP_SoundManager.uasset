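; Sound manager Blueprint that plays music tied to a one-time player achievement.
; A fast looping timer watches BP_SwordCharacter for a lit torch or a specific equipped weapon, then after a short delay plays a discovery cue, decrements SticksQuantity and sets AchievementUnlocked.
; A slower timer waits on that flag, then plays two music tracks once each, separated by random delays, with DoOnce preventing repeats.
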(event Custom|CheckForAchievement
  (if (or (Variables|/Game/FPSwordAndShield/Blueprints/BP_SwordCharacter.BP_SwordCharacter_C|GetTorchLit (stale EventBeginPlay _asbp_sword_character)) (Utilities|Enum|Equal(Enum) (Variables|/Game/FPSwordAndShield/Blueprints/BP_SwordCharacter.BP_SwordCharacter_C|GetEquippedWeapon (stale EventBeginPlay _asbp_sword_character)) "NewEnumerator1"))
    (Utilities|FlowControl|DoOnce false
      (:Completed
        (Utilities|FlowControl|Delay 2.0)
        (Audio|PlaySound2D "/Game/Audio/MusicDiscovered.MusicDiscovered" 0.3 1.0 0.0 0 0)
        (Math|Integer|DecrementInt (Variables|/Game/FPSwordAndShield/Blueprints/BP_SwordCharacter.BP_SwordCharacter_C|GetSticksQuantity (stale EventBeginPlay _asbp_sword_character))
          (:%20%20
            (Variables|Default|SetAchievementUnlocked true)))))))

(event Custom|PlayNextSound
  (if (Variables|Default|GetAchievementUnlocked)
    (Utilities|FlowControl|DoOnce false
      (:Completed
        (Utilities|FlowControl|Delay (Math|Random|RandomFloatinRange 6e+01 1.2e+02))
        (Audio|PlaySound2D "/Game/Audio/music_1.music_1" 0.5 1.0 0.0 0 0)
        (Utilities|FlowControl|Delay (Math|Random|RandomFloatinRange 6e+01 1.2e+02))
        (Audio|PlaySound2D "/Game/Audio/music_2.music_2" 0.5 1.0 0.0 0 0)))))

(event EventBeginPlay
  (bind _asbp_sword_character (Utilities|Casting|CastToBP_SwordCharacter (Game|GetPlayerCharacter 0)))
  (Utilities|Time|SetTimerbyEvent (delegate Custom|CheckForAchievement) 0.2 true)
  (Utilities|Time|SetTimerbyEvent (delegate Custom|PlayNextSound) 15.0 true))

(fn ConstructionScript)