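; BP_Raft is an actor that runs a game-over sequence as soon as it begins play.
; It casts the player pawn to BP_SwordCharacter, then plays a timeline that eases global time dilation toward zero while damping the character's ActionValueX and ActionValueY.
; A DoOnce on the timeline's update creates the WB_GameOver widget and adds it to the viewport a single time.
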(event EventBeginPlay
  (bind _asbp_sword_character (Utilities|Casting|CastToBP_SwordCharacter (Game|GetPlayerCharacter 0)))
  (bind _newtrack_0 (Timeline|Timeline Play)
    (:Update
      (Utilities|Time|SetGlobalTimeDilation (Math|Float|Lerp 1.0 0.0 _newtrack_0))
      (Variables|/Game/FPSwordAndShield/Blueprints/BP_SwordCharacter.BP_SwordCharacter_C|SetAction%20Value%20X _asbp_sword_character (Math|Float|Lerp (Variables|/Game/FPSwordAndShield/Blueprints/BP_SwordCharacter.BP_SwordCharacter_C|GetAction%20Value%20X _asbp_sword_character) 0.0 _newtrack_0))
      (Variables|/Game/FPSwordAndShield/Blueprints/BP_SwordCharacter.BP_SwordCharacter_C|SetAction%20Value%20Y _asbp_sword_character (Math|Float|Lerp (Variables|/Game/FPSwordAndShield/Blueprints/BP_SwordCharacter.BP_SwordCharacter_C|GetAction%20Value%20Y _asbp_sword_character) 0.0 _newtrack_0))
      (Utilities|FlowControl|DoOnce false
        (:Completed
          (bind _returnvalue (UserInterface|CreateWidget "/Game/UI/Menus/WB_GameOver.WB_GameOver_C"))
          (UserInterface|Viewport|AddtoViewport _returnvalue 0))))))

(fn ConstructionScript)