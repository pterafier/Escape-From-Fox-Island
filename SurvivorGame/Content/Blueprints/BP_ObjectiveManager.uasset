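; BP_ObjectiveManager unlocks the player's axe and torch once enough crafting materials are collected.
; On BeginPlay it caches the BP_SwordCharacter player and starts looping timers that poll its resource counters.
; The axe requires rocks and sticks at the crafting cost, while the torch requires a stick and fiber.
; Each check sets the unlock flag on the character, then clears its own timer.
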(event Custom|UnlockAxe
  (bind _as_bp_sword_character (Variables|Default|GetAs%20BP%20Sword%20Character))
  (if (and (>= (Variables|/Game/FPSwordAndShield/Blueprints/BP_SwordCharacter.BP_SwordCharacter_C|GetRockCounter _as_bp_sword_character) (Variables|Default|GetAxeCraftingCost)) (>= (Variables|/Game/FPSwordAndShield/Blueprints/BP_SwordCharacter.BP_SwordCharacter_C|GetSticksQuantity _as_bp_sword_character) (Variables|Default|GetAxeCraftingCost)))
    (Variables|/Game/FPSwordAndShield/Blueprints/BP_SwordCharacter.BP_SwordCharacter_C|SetAxeUnlocked (Variables|Default|GetAs%20BP%20Sword%20Character) true)
    (Utilities|Time|ClearandInvalidateTimerbyHandle (stale EventBeginPlay _returnvalue))))

(event Custom|UnlockTorch
  (bind _as_bp_sword_character (Variables|Default|GetAs%20BP%20Sword%20Character))
  (if (and (>= (Variables|/Game/FPSwordAndShield/Blueprints/BP_SwordCharacter.BP_SwordCharacter_C|GetSticksQuantity _as_bp_sword_character) 1) (>= (Variables|/Game/FPSwordAndShield/Blueprints/BP_SwordCharacter.BP_SwordCharacter_C|GetFiber _as_bp_sword_character) 1))
    (Variables|/Game/FPSwordAndShield/Blueprints/BP_SwordCharacter.BP_SwordCharacter_C|SetTorchUnlocked _as_bp_sword_character true)
    (Utilities|Time|ClearandInvalidateTimerbyHandle (stale EventBeginPlay _returnvalue_2))))

(event EventBeginPlay
  (bind _asbp_sword_character (Utilities|Casting|CastToBP_SwordCharacter (Game|GetPlayerCharacter 0)))
  (Variables|Default|SetAs%20BP%20Sword%20Character _asbp_sword_character)
  (bind _returnvalue (Utilities|Time|SetTimerbyEvent (delegate Custom|UnlockAxe) 0.2 true))
  (bind _returnvalue_2 (Utilities|Time|SetTimerbyEvent (delegate Custom|UnlockTorch) 0.2 true)))

(fn ConstructionScript)